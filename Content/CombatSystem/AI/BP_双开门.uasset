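; Double sliding door actor (双开门) whose Right and Left panels move apart along their local Y axis.
; BeginPlay runs the parent logic, then caches each panel's starting relative location and derives an open position offset in opposite directions.
; The AnimationtoDoor event lerps both panels between these positions using its Time input as alpha, without sweep.
; Nothing in this graph triggers that event or generates the alpha.
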(event EventBeginPlay
  (|CallParentFunction)
  (bind _output_get (Variables|Default|SetDoor%20Location%20R (Variables|/Script/Engine.SceneComponent|GetRelativeLocation (Variables|Default|GetRight))))
  (Variables|Default|SetDoor%20End%20R (+ _output_get "0.000000,-200.000000,0.000000"))
  (bind _output_get_2 (Variables|Default|SetDoor%20Location%20L (Variables|/Script/Engine.SceneComponent|GetRelativeLocation (Variables|Default|GetLeft))))
  (Variables|Default|SetDoor%20End%20L (+ _output_get_2 "0.000000,200.000000,0.000000")))

(event Collision|EventActorBeginOverlap
  (params (OtherActor :type Actor%20Object%20Reference))
  (|CallParentFunction OtherActor) ; 此节点被禁用，将不会被调用。\n从引脚连出引线来编译功能。
)

(event EventTick
  (params (DeltaSeconds :type Float%20%28single-precision%29))
  (|CallParentFunction DeltaSeconds) ; 此节点被禁用，将不会被调用。\n从引脚连出引线来编译功能。
)

(event EventAnimationtoDoor
  (params (Time :type Float%20%28double-precision%29))
  (Transformation|SetRelativeLocation (Variables|Default|GetRight) (Math|Vector|Lerp(Vector) (Variables|Default|GetDoor%20Location%20R) (Variables|Default|GetDoor%20End%20R) Time) false false)
  (Transformation|SetRelativeLocation (Variables|Default|GetLeft) (Math|Vector|Lerp(Vector) (Variables|Default|GetDoor%20Location%20L) (Variables|Default|GetDoor%20End%20L) Time) false false))

(fn ConstructionScript
  (|CallParentFunction))