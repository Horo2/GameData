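; Base combat NPC character with a camera-facing health bar, timeline turning toward the player and death handling.
; Hit feedback from the status component drives the behaviour component, switching off data-table-listed services unless super armour (霸体) is on.
; Airborne hits juggle the NPC by briefly hovering it before the player, while a sphere-trace loop detects landing for get-up or death.
; Tick also teleports NPCs stuck off the navmesh to a random reachable point.
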(event AttackFeedbackNotification(C_NPC_Status_Component)
  (params (Actor :type Actor%20Object%20Reference))
  (bind _returnvalue (Game|GetPlayerCharacter 0))
  (bind _npc_behaviourallogic_component (Variables|Default|GetNPC%20BehaviouralLogic%20Component))
  (bind _npc_behaviour (Default|GetNPCBehaviour _npc_behaviourallogic_component))
  ;[0 0 0] 攻击反馈
  (if (or (Utilities|Enum|Equal(Enum) _npc_behaviour "NewEnumerator17") (Utilities|Enum|Equal(Enum) _npc_behaviour "NewEnumerator18"))
    ;;[1 1 1] NPC在掉落时被连击
    (if (> (.currenthp (Variables|/Game/CombatSystem/AI/NPC/C_NPC_Status_Component.C_NPC_Status_Component_C|GetNPC%20Basic%20Data (Variables|Default|GetC_NPC_Status_Component))) 0.0)
      (Animation|Montage|PlayMontage (Variables|Character|GetMesh) "/Game/CombatSystem/Enemy_anim/Elite_B/DMG/击飞.击飞" 1.0 0.0 "掉落"
        (:then
          (Transformation|SetActorLocation (+ (Transformation|GetActorLocation _returnvalue) (* (Transformation|GetActorForwardVector _returnvalue) (Math|Conversions|ToFloat(Integer) "100"))) false false)
          (Pawn|Components|CharacterMovement|SetMovementMode (Variables|Character|GetCharacterMovement) "MOVE_Flying" 0)
          (Physics|SetEnableGravity (Variables|Collision|GetCapsuleComponent) false)
          (Components|Movement|StopMovementImmediately (Variables|Character|GetCharacterMovement))
          (Default|SetNPCBehaviour (Variables|Default|GetNPC%20BehaviouralLogic%20Component) "NewEnumerator18")
          (Utilities|FlowControl|RetriggerableDelay 0.5))))
    (Pawn|Components|CharacterMovement|SetMovementMode (Variables|Character|GetCharacterMovement) "MOVE_Walking" 0)
    (Physics|SetEnableGravity (Variables|Collision|GetCapsuleComponent) true)
    (Default|SetNPCBehaviour (Variables|Default|GetNPC%20BehaviouralLogic%20Component) "NewEnumerator17")
    (elif (Variables|Default|Get霸体)
      (if (not (> (.currenthp (Variables|/Game/CombatSystem/AI/NPC/C_NPC_Status_Component.C_NPC_Status_Component_C|GetNPC%20Basic%20Data (Variables|Default|GetC_NPC_Status_Component))) 0.0))
        (CallFunction|死亡))
      (else
        (CallFunction|设置所有服务是否激活 false)
        (Default|SetNPCBehaviour (Variables|Default|GetNPC%20BehaviouralLogic%20Component) "NewEnumerator14")
        (CallFunction|ActivateEnemyService false)))))

(event Custom|死亡
  ;[1 1 1] NPC死亡逻辑
  (Collision|SetActorEnableCollision false)
  (Default|SetNPCBehaviour (Variables|Default|GetNPC%20BehaviouralLogic%20Component) "NewEnumerator16")
  (Variables|Default|SetNPC%20Death true)
  (bind _outcolumnnames (Class|DataTableFunctionLibrary|GetDataTableColumnNames "/Game/CombatSystem/AI/NPC/NPCData/Service_DataTable.Service_DataTable"))
  (for _array_element _outcolumnnames
    (bind _returnvalue (Utilities|GetDataTableRow "/Game/CombatSystem/AI/NPC/NPCData/Service_DataTable.Service_DataTable" _array_element)
      (:then
        (Default|SetActicationService (Variables|Default|GetNPC%20BehaviouralLogic%20Component) false (.服务名 _returnvalue)))))
  (CallFunction|ActivateEnemyService false)
  (bind _notifyname (Animation|Montage|PlayMontage (Variables|Character|GetMesh) (Variables|动画蒙太奇|Get死亡动画蒙太奇))
    (:OnNotifyBegin
      (switch name _notifyname
        (:死亡
          (Default|CallAIDeath)
          (Actor|DestroyActor))))))

(event Custom|Stop%20Rotation%20Animation
  (bind _returnvalue (Game|GetPlayerCharacter 0))
  ;[0 0 0] 转身动画
  (bind _新建轨道_0 (Timeline|时间轴 Stop)
    (:Update
      (Utilities|IsValid _returnvalue
        (:Is%20Valid
          (Transformation|SetActorRotation self (Math|Rotator|MakeRotator 0.0 0.0 (Math|Float|Lerp (Variables|Default|GetIteslf%20Rotation) (.yaw (Math|Rotator|FindLookatRotation (Transformation|GetActorLocation) (Transformation|GetActorLocation _returnvalue))) _新建轨道_0))))))
    (:Finished
      (CallFunction|PlayeRotationAnimation))))

(event Custom|Activate%20Enemy%20Service
  (params (Activate? :type Boolean))
  (if Activate?
    (Variables|Default|SetbUseControllerRotationYaw false)
    (CallFunction|PlayeRotationAnimation)
    (else
      (Variables|Default|SetbUseControllerRotationYaw true)
      (CallFunction|StopRotationAnimation))))

(event Custom|Attack)

(event Custom|Playe%20Rotation%20Animation
  (bind _returnvalue (Game|GetPlayerCharacter 0))
  ;[0 0 0] 转身动画
  (Variables|Default|SetIteslf%20Rotation (.yaw (Transformation|GetActorRotation)))
  (bind _新建轨道_0 (Timeline|时间轴 Play)
    (:Update
      (Utilities|IsValid _returnvalue
        (:Is%20Valid
          (Transformation|SetActorRotation self (Math|Rotator|MakeRotator 0.0 0.0 (Math|Float|Lerp (Variables|Default|GetIteslf%20Rotation) (.yaw (Math|Rotator|FindLookatRotation (Transformation|GetActorLocation) (Transformation|GetActorLocation _returnvalue))) _新建轨道_0))))))
    (:Finished
      (CallFunction|PlayeRotationAnimation))))

(event Custom|受击结束通知)

(event Custom|NPC掉落判定
  (bind _returnvalue (Transformation|GetActorLocation))
  ;[0 0 0] NPC 掉落判定
  (Animation|Montage|PlayMontage (Variables|Character|GetMesh) "/Game/CombatSystem/Enemy_anim/Elite_B/DMG/空中掉落.空中掉落" 1.0 0.0 "掉落"
    (:then
      (bind _returnvalue_2 (Collision|SphereTraceForObjects _returnvalue (+ _returnvalue (* (Transformation|GetActorUpVector) (* (Math|Conversions|ToFloat(Integer) "110") -1.0))) 1e+01 (Utilities|Array|MakeArray "ObjectTypeQuery1" "ObjectTypeQuery2") false (Utilities|Array|MakeArray self) "ForDuration" :!label _label)) ; 检测NPC是否落地
      (if _returnvalue_2
        (if (Utilities|Enum|Equal(Enum) (Default|GetNPCBehaviour (Variables|Default|GetNPC%20BehaviouralLogic%20Component)) "NewEnumerator18")
          (Utilities|FlowControl|Delay 0.1 :!label _label_2)
          (goto _label)
          (else
            (Variables|/Game/CombatSystem/AI/NPC/C_NPC_Status_Component.C_NPC_Status_Component_C|Set无敌状态 (Variables|Default|GetC_NPC_Status_Component) true)
            (bind _notifyname (Animation|Montage|PlayMontage (Variables|Character|GetMesh) "/Game/CombatSystem/Enemy_anim/Elite_B/DMG/掉落结束.掉落结束")
              (:OnNotifyBegin
                (switch name _notifyname
                  (:伤亡判定
                    (if (> (.currenthp (Variables|/Game/CombatSystem/AI/NPC/C_NPC_Status_Component.C_NPC_Status_Component_C|GetNPC%20Basic%20Data (Variables|Default|GetC_NPC_Status_Component))) 0.0)
                      (Animation|Montage|PlayMontage (Variables|Character|GetMesh) "/Game/CombatSystem/Enemy_anim/Elite_B/DMG/掉落结束站起.掉落结束站起"
                        (:OnCompleted
                          (Variables|Default|Set中断攻击 false)
                          (Variables|Default|Set正在被击飞 false)
                          (Variables|/Game/CombatSystem/AI/NPC/C_NPC_Status_Component.C_NPC_Status_Component_C|Set无敌状态 (Variables|Default|GetC_NPC_Status_Component) false)
                          (CallFunction|受击结束通知)))
                      (else
                        (CallFunction|ActivateEnemyService false)
                        (Default|CallAIDeath)
                        (Actor|DestroyActor)))))))))
        (else
          (goto _label_2))))))

(event Custom|卡死自救
  (bind _returnvalue (Transformation|GetActorLocation))
  (bind _npc_behaviourallogic_component (Variables|Default|GetNPC%20BehaviouralLogic%20Component))
  (bind _npc_behaviour (Default|GetNPCBehaviour _npc_behaviourallogic_component))
  (bind (_randomlocation _returnvalue_2) (AI|Navigation|GetRandomReachablePointinRadius _returnvalue 8e+02 0 "/Script/AIModule.NavFilter_AIControllerDefault"))
  ;[1 0 0] 卡死自救逻辑
  (if (not (.ReturnValue (AI|Navigation|ProjectPointtoNavigation (Transformation|GetActorLocation) 0 0 "0, 0, 0")))
    (Utilities|FlowControl|Delay 2.0)
    (if (not (.ReturnValue (AI|Navigation|ProjectPointtoNavigation (Transformation|GetActorLocation) 0 0 "0, 0, 0")))
      (if (not (or (Utilities|Enum|Equal(Enum) _npc_behaviour "NewEnumerator17") (Utilities|Enum|Equal(Enum) _npc_behaviour "NewEnumerator18")))
        (Utilities|FlowControl|Delay 6.0)
        (if _returnvalue_2 :!label _label
          (Transformation|SetActorLocation _randomlocation false false)
          (Development|PrintString "自救" true true "(R=0.001268,G=1.000000,B=0.000000,A=1.000000)" 31231.0)
          (else
            (Utilities|FlowControl|Delay 0.2)
            (goto _label)))))))

(event EventBeginPlay
  ;[1 0 0] 将NPC同步给血条
  (bind _aswbp_npcblood_strip (Utilities|Casting|CastToWBP_NPCBloodStrip (UserInterface|GetWidget (Variables|Default|GetNPC%20Blood%20Strip))))
  (Variables|/Game/CombatSystem/AI/NPC/UMG/WBP_NPCBloodStrip.WBP_NPCBloodStrip_C|SetNPC%20Character _aswbp_npcblood_strip self))

(event Collision|EventActorBeginOverlap
  (params (OtherActor :type Actor%20Object%20Reference)))

(event EventTick
  (params (DeltaSeconds :type Float%20%28single-precision%29))
  (Transformation|SetWorldRotation (Variables|Default|GetNPC%20Blood%20Strip) (Math|Rotator|FindLookatRotation (Transformation|GetActorLocation) (Transformation|GetActorLocation (Variables|/Script/Engine.PlayerController|GetPlayerCameraManager (Game|GetPlayerController 0)))) false false)
  (CallFunction|卡死自救))

(event EventDestroyed
  ;[0 0 0] 攻击反馈
  (Default|CallAIDeath))

(fn ConstructionScript)

(fn 设置所有服务是否激活
  (params (Activation :type Boolean))
  (bind _outcolumnnames (Class|DataTableFunctionLibrary|GetDataTableColumnNames "/Game/CombatSystem/AI/NPC/NPCData/Service_DataTable.Service_DataTable"))
  (for _array_element _outcolumnnames
    (bind _returnvalue (Utilities|GetDataTableRow "/Game/CombatSystem/AI/NPC/NPCData/Service_DataTable.Service_DataTable" _array_element)
      (:then
        (Default|SetActicationService (Variables|Default|GetNPC%20BehaviouralLogic%20Component) Activation (.服务名 _returnvalue))))))

(fn OnRep霸体
  (if (not (Variables|Default|Get霸体))
    (if (not (> (.currenthp (Variables|/Game/CombatSystem/AI/NPC/C_NPC_Status_Component.C_NPC_Status_Component_C|GetNPC%20Basic%20Data (Variables|Default|GetC_NPC_Status_Component))) 0.0))
      (CallFunction|死亡))))

(fn CanRecieveDamage
  (return (Variables|Default|GetRecieve%20Damage)))

(fn GetDesiredRotation
  (return "0, 0, 0"))