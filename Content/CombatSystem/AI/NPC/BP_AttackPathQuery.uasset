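; Short-lived AI query actor that finds an attack position near a target actor, judging by its name and CombatSystem NPC folder.
; A looping timer steps along a spline, sphere-tracing along its right vector and collecting hit or end points beyond a minimum distance, discarding NPC hits.
; It then picks the point closest to the query target, traces downward for ground, reports the result through an EnquiryCompleted event and destroys itself.
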(event Custom|数据处理
  (for _array_element (Variables|Default|Get符合数据位置信息)
    (if (< (Math|Vector|Distance(Vector) _array_element (Transformation|GetActorLocation (Variables|Default|Get查询对象))) (Variables|Default|Get判断最远距离))
      (Variables|Default|Set判断最远距离 (Math|Vector|Distance(Vector) _array_element (Transformation|GetActorLocation (Variables|Default|Get查询对象))))
      (Variables|Default|Set最近的点 _array_element)))
  (bind (_outhit _returnvalue) (Collision|SphereTraceForObjects (Variables|Default|Get最近的点) (+ (Variables|Default|Get最近的点) (Math|Vector|MakeVector (.X (Math|Vector|BreakVector (Variables|Default|Get最近的点))) (.Y (Math|Vector|BreakVector (Variables|Default|Get最近的点))) (- (.Z (Math|Vector|BreakVector (Variables|Default|Get最近的点))) (Math|Conversions|ToFloat(Integer) "999999999999")))) 4e+01 (Utilities|Array|MakeArray "ObjectTypeQuery1" "ObjectTypeQuery2") false 0 "None"))
  (if _returnvalue
    (Default|CallEnquiryCompletedEvent (.Location (Collision|BreakHitResult _outhit)))
    (Actor|DestroyActor)
    (else
      (Default|CallEnquiryCompletedEvent (Variables|Default|Get最近的点))
      (Actor|DestroyActor))))

(event Custom|检测周边
  (bind _spline (Variables|Default|GetSpline))
  (Variables|Default|SetTime (+ (Variables|Default|GetTime) 0.01))
  (if (>= (Variables|Default|GetTime) 1.0)
    (Utilities|Time|PauseTimerbyHandle (Variables|Default|Get检测定时器))
    (CallFunction|数据处理)
    (else
      (bind (_outhit _returnvalue) (Collision|SphereTraceForObjects (Spline|GetLocationatTime _spline (Variables|Default|GetTime) "World" false) (+ (Spline|GetLocationatTime _spline (Variables|Default|GetTime) "World" false) (* (Class|SplineComponent|GetRightVectoratTime _spline (Variables|Default|GetTime) "World" false) (Variables|Default|Get检测长度))) 4e+01 (Utilities|Array|MakeArray "ObjectTypeQuery1" "ObjectTypeQuery2" "ObjectTypeQuery3" "ObjectTypeQuery4" "ObjectTypeQuery5" "ObjectTypeQuery6" "ObjectTypeQuery7") false (Utilities|Array|MakeArray (Game|GetPlayerCharacter 0)) "None"))
      (if _returnvalue
        (Utilities|Casting|CastToBP_NPC_Character (.HitActor (Collision|BreakHitResult _outhit))
          (:CastFailed
            (if (>= (Math|Vector|Distance(Vector) (.Location (Collision|BreakHitResult _outhit)) (Transformation|GetActorLocation)) (Variables|Default|Get最近距离))
              (Utilities|Array|Add (Variables|Default|Get符合数据位置信息) (.Location (Collision|BreakHitResult _outhit))))))
        (elif (>= (Math|Vector|Distance(Vector) (+ (Spline|GetLocationatTime _spline (Variables|Default|GetTime) "World" false) (* (Class|SplineComponent|GetRightVectoratTime _spline (Variables|Default|GetTime) "World" false) (Variables|Default|Get检测长度))) (Transformation|GetActorLocation)) (Variables|Default|Get最近距离))
          (Utilities|Array|Add (Variables|Default|Get符合数据位置信息) (+ (Spline|GetLocationatTime _spline (Variables|Default|GetTime) "World" false) (* (Class|SplineComponent|GetRightVectoratTime _spline (Variables|Default|GetTime) "World" false) (Variables|Default|Get检测长度)))))))))

(event EventBeginPlay
  (bind _returnvalue (Utilities|Time|SetTimerbyEvent (delegate Custom|检测周边) 0.001 true))
  (Variables|Default|Set检测定时器 _returnvalue))

(fn ConstructionScript)