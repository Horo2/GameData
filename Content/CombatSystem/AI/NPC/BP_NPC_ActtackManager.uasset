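; NPC attack manager that limits how many BP_NPC_Character enemies hold an attack permit at once, aiming for three.
; From BeginPlay it loops every 0.2 seconds, gathering all NPCs that accept the manager, counting permit holders and listing the rest as candidates.
; Free slots go to random candidates through SetAttackLicence on NPCBehaviouralLogicComponent; picks can repeat, and permits are never revoked here.
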(event Custom|给予攻击许可
  (bind _outactors (Actor|GetAllActorsOfClass "/Game/CombatSystem/AI/NPC/BP_NPC_Character.BP_NPC_Character_C"))
  (Variables|Default|SetNPC%20Character%20Data _outactors)
  (for _array_element (Variables|Default|GetNPC%20Character%20Data)
    (if (Variables|/Game/CombatSystem/AI/NPC/BP_NPC_Character.BP_NPC_Character_C|GetAcceptance%20Attack%20Manager _array_element)
      (if (.AttackPermit (Utilities|Struct|BreakNPC_CharacterData_Struct (Variables|/Game/CombatSystem/AI/NPC/NPCData/C_NPC_BehaviouralLogic_Component.C_NPC_BehaviouralLogic_Component_C|GetNPC%20Data (Variables|/Game/CombatSystem/AI/NPC/BP_NPC_Character.BP_NPC_Character_C|GetNPC%20BehaviouralLogic%20Component _array_element))))
        (Math|Integer|IncrementInt (Variables|Default|Get已允许攻击的人数))
        (else
          (Utilities|Array|Add (Variables|Default|GetCan%20Carry%20Out%20Attack%20NPC) _array_element)))))
  (if (< (Variables|Default|Get已允许攻击的人数) 3)
    (for _index (range 0 (- (- 3 (Variables|Default|Get已允许攻击的人数)) 1))
      (if (<= _index (- (Utilities|Array|Length (Variables|Default|GetCan%20Carry%20Out%20Attack%20NPC)) 1))
        (Default|SetAttackLicence (Variables|/Game/CombatSystem/AI/NPC/BP_NPC_Character.BP_NPC_Character_C|GetNPC%20BehaviouralLogic%20Component (Utilities|Array|Get(acopy) (Variables|Default|GetCan%20Carry%20Out%20Attack%20NPC) (Math|Random|RandomIntegerinRange 0 (- (Utilities|Array|Length (Variables|Default|GetCan%20Carry%20Out%20Attack%20NPC)) 1)))) true)))
    (CallFunction|重置给予攻击许可)
    (else
      (CallFunction|重置给予攻击许可))))

(event Custom|重置给予攻击许可
  (Utilities|FlowControl|Delay 0.2)
  (Utilities|Array|Clear (Variables|Default|GetCan%20Carry%20Out%20Attack%20NPC))
  (Variables|Default|Set已允许攻击的人数 0)
  (Utilities|Array|Clear (Variables|Default|GetNPC%20Character%20Data))
  (CallFunction|给予攻击许可))

(event EventBeginPlay
  (CallFunction|给予攻击许可))

(event Collision|EventActorBeginOverlap
  (params (OtherActor :type Actor%20Object%20Reference)))

(event EventTick
  (params (DeltaSeconds :type Float%20%28single-precision%29)))

(fn ConstructionScript)