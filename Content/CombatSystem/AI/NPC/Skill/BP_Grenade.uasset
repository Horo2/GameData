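; Grenade actor that damages the player with a timed area explosion, using a configurable mesh set on BeginPlay.
; The 激活手雷 (activate grenade) event shows the Sphere, waits a fuse delay, then runs a single-hit Pawn sphere trace and calls TakeDamage on a Player-tagged hit's BP_StatsComponent.
; It then plays sound, hides the visuals, triggers RemoteExplosion, and destroys itself when that effect finishes.
; Overlap-triggered damage logic is left unconnected.
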(event OnComponentBeginOverlap(StaticMesh)
  (params (OverlappedComponent :type Primitive%20Component%20Object%20Reference) (OtherActor :type Actor%20Object%20Reference) (OtherComp :type Primitive%20Component%20Object%20Reference) (OtherBodyIndex :type Integer) (bFromSweep :type Boolean) (SweepResult :type Hit%20Result%20Structure%20%28by%20ref%29)))

(event OnSystemFinished(Remote_Explosion)
  (params (PSystem :type Particle%20System%20Component%20Object%20Reference))
  (Actor|DestroyActor))

(event Custom|激活手雷
  (bind _staticmesh (Variables|Default|GetStaticMesh))
  (bind _returnvalue (Transformation|GetWorldLocation _staticmesh))
  (Rendering|SetVisibility (Variables|Default|GetSphere) true true)
  (Utilities|FlowControl|Delay 2.5)
  (bind (_outhit _returnvalue_2) (Collision|SphereTraceForObjects _returnvalue _returnvalue 3e+02 (Utilities|Array|MakeArray "ObjectTypeQuery3") false (Utilities|Array|MakeArray self) "ForDuration"))
  (if _returnvalue_2
    (if (Actor|ActorHasTag (.HitActor (Collision|BreakHitResult _outhit)) "Player")
      (Default|TakeDamage (Actor|GetComponentbyClass (.HitActor (Collision|BreakHitResult _outhit)) "/Game/CombatSystem/Blueprints/Components/BP_StatsComponent.BP_StatsComponent_C") (Variables|Default|GetIn%20Damage) 0.0 self true "NewEnumerator6")))
  (Audio|SpawnSoundatLocation "/Game/CombatSystem/enemy_sfx/Remote/ShouLei_BaoZha.ShouLei_BaoZha" (Transformation|GetWorldLocation (Variables|Default|GetStaticMesh)) "0, 0, 0" 1.0 1.0 0.0 0 0)
  (Transformation|SetWorldLocation (Variables|Default|GetRemote_Explosion) (Transformation|GetWorldLocation (Variables|Default|GetStaticMesh)) false false)
  (Rendering|SetVisibility (Variables|Default|GetStaticMesh) false false)
  (Components|Activation|SetActive (Variables|Default|GetRemote_Explosion) true true))

(event EventBeginPlay
  (Components|StaticMesh|SetStaticMesh (Variables|Default|GetStaticMesh) (Variables|Default|GetBombs%20Static%20Mesh))
  (Rendering|SetVisibility (Variables|Default|GetSphere) false false))

(event Collision|EventActorBeginOverlap
  (params (OtherActor :type Actor%20Object%20Reference)))

(event EventTick
  (params (DeltaSeconds :type Float%20%28single-precision%29)))

(fn ConstructionScript)