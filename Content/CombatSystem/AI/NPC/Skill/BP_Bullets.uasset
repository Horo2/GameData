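; BP_Bullets is a projectile for NPC ranged skills that damages the player.
; On BeginPlay it applies its mesh and fire effect, then turns once toward the player's position, without homing.
; Each Tick it moves along its arrow's forward vector and runs a sphere trace in place, with debug drawing, rather than using overlap events.
; Any hit destroys it, first applying damage through BP_StatsComponent if the actor is tagged Player.
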(event OnComponentBeginOverlap(Box)
  (params (OverlappedComponent :type Primitive%20Component%20Object%20Reference) (OtherActor :type Actor%20Object%20Reference) (OtherComp :type Primitive%20Component%20Object%20Reference) (OtherBodyIndex :type Integer) (bFromSweep :type Boolean) (SweepResult :type Hit%20Result%20Structure%20%28by%20ref%29)))

(event EventBeginPlay
  (Components|StaticMesh|SetStaticMesh (Variables|Default|GetRemote_Bullet) (Variables|Default|GetBullets%20Stataic%20Mehs))
  (Class|NiagaraComponent|SetAsset (Variables|Default|GetRemote_NormalAttack_Fire) (Variables|Default|GetIn%20Asset) true)
  (Components|Activation|SetActive (Variables|Default|GetRemote_NormalAttack_Fire) true true)
  (Transformation|SetActorRotation (Math|Rotator|FindLookatRotation (Transformation|GetActorLocation) (Transformation|GetActorLocation (Game|GetPlayerCharacter 0)))))

(event Collision|EventActorBeginOverlap
  (params (OtherActor :type Actor%20Object%20Reference)))

(event EventTick
  (params (DeltaSeconds :type Float%20%28single-precision%29))
  (bind _returnvalue (Transformation|GetActorLocation))
  (Transformation|AddActorWorldOffset (* (Math|Vector|GetForwardVector (Variables|Default|GetArrow)) (Variables|Default|GetBullets%20Speed)))
  (bind (_outhit _returnvalue_2) (Collision|SphereTraceByChannel _returnvalue _returnvalue 3e+01 "TraceTypeQuery1" false (Utilities|Array|MakeArray (Variables|Default|GetActor)) "ForDuration"))
  (if _returnvalue_2
    (if (Actor|ActorHasTag (.HitActor (Collision|BreakHitResult _outhit)) "Player")
      (Default|TakeDamage (Actor|GetComponentbyClass (.HitActor (Collision|BreakHitResult _outhit)) "/Game/CombatSystem/Blueprints/Components/BP_StatsComponent.BP_StatsComponent_C") (Variables|Default|GetIn%20Damage) 0.0 self true "NewEnumerator0")
      (Actor|DestroyActor)
      (else
        (Actor|DestroyActor)))))

(fn ConstructionScript)