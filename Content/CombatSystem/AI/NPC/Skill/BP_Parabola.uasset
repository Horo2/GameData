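; BP_Parabola is an NPC skill actor that lobs a grenade along an arc toward EndPosition.
; On BeginPlay it builds a spline from a Bezier curve, peaking midway with height scaled by distance, and spawns BP_Grenade with InDamage.
; Tick moves the grenade along the spline, sphere-tracing after a short delay.
; On a hit or path end, it enables grenade physics, activates it and destroys itself.
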(event Custom|Explosive%20Event_事件
  (Actor|DestroyActor (Variables|Default|GetBombs))
  (Actor|DestroyActor))

(event EventBeginPlay
  (bind _sphere (Variables|Default|GetSphere))
  (bind _relativelocation (Variables|/Script/Engine.SceneComponent|GetRelativeLocation _sphere))
  (Transformation|SetWorldLocation (Variables|Default|GetSphere) (Variables|Default|GetEnd%20Position) false false)
  (Utilities|Array|Add (Variables|Default|GetSrc) (Math|Vector2D|MakeVector2D 0.0 0.0))
  (Utilities|Array|Add (Variables|Default|GetSrc) (Math|Vector2D|MakeVector2D (.x (/ (+ "" (Variables|/Script/Engine.SceneComponent|GetRelativeLocation (Variables|Default|GetSphere))) (Math|Conversions|ToFloat(Integer) "2"))) (Math|Vector|Distance(Vector) "0, 0, 0" (Variables|/Script/Engine.SceneComponent|GetRelativeLocation (Variables|Default|GetSphere)))))
  (Utilities|Array|Add (Variables|Default|GetSrc) (Math|Vector2D|MakeVector2D (.x _relativelocation) (.z _relativelocation)))
  (bind _returnvalue (Class|BerzierCurveComponent|BerzierCurve (Variables|Default|GetBerzierCurve) (Variables|Default|GetSrc)))
  (Spline|ClearSplinePoints (Variables|Default|GetSpline) true)
  (for _array_element _returnvalue
    (Spline|AddSplinePoint (Variables|Default|GetSpline) (Math|Vector|MakeVector (.x _array_element) 0.0 (.y _array_element)) "Local" false))
  (Spline|UpdateSpline (Variables|Default|GetSpline))
  (bind _returnvalue_2 (Game|SpawnActorfromClass "/Game/CombatSystem/AI/NPC/Skill/BP_Grenade.BP_Grenade_C" (Math|Transform|MakeTransform "0, 0, 0" "0, 0, 0" "1.000000,1.000000,1.000000") "Undefined" "MultiplyWithRoot" 0 "/Game/CombatSystem/Enemy_VFX/Remote_VFX/Remote_Grenade.Remote_Grenade" (Variables|Default|GetIn%20Damage) 0))
  (bind _output_get (Variables|Default|SetBombs _returnvalue_2))
  (EventDispatchers|AssignExplosiveEvent _output_get (delegate Custom|Explosive%20Event_事件))
  (Variables|Default|SetStat%20Runing%20Bombs%20Animation true))

(event EventTick
  (params (DeltaSeconds :type Float%20%28single-precision%29))
  (bind _bombs (Variables|Default|GetBombs))
  (bind _bombs_2 (Variables|Default|GetBombs))
  (bind _returnvalue (Transformation|GetActorLocation _bombs))
  (if (Variables|Default|GetStat%20Runing%20Bombs%20Animation)
    (bind _output_get (Variables|Default|SetRuning%20Time (+ (* DeltaSeconds (Variables|Default|GetRuning%20Speed)) (Variables|Default|GetRuning%20Time))))
    (Development|PrintString (Utilities|String|ToString(Float) _output_get))
    (Transformation|SetActorLocation (Variables|Default|GetBombs) (Spline|GetLocationatTime (Variables|Default|GetSpline) (Variables|Default|GetRuning%20Time) "World" false) false false)
    (if (>= (Variables|Default|GetRuning%20Time) 0.2)
      (bind _returnvalue_2 (Collision|SphereTraceForObjects _returnvalue _returnvalue 2e+01 (Utilities|Array|MakeArray "ObjectTypeQuery1" "ObjectTypeQuery2") false 0 "None"))
      (if _returnvalue_2
        (Physics|SetSimulatePhysics (Variables|/Game/CombatSystem/AI/NPC/Skill/BP_Grenade.BP_Grenade_C|GetStaticMesh _bombs_2) true :!label _label)
        (Default|激活手雷 _bombs_2)
        (Actor|DestroyActor)
        (else
          (if (>= (Variables|Default|GetRuning%20Time) 1.0) :!label _label_2
            (goto _label))))
      (else
        (goto _label_2)))))

(fn ConstructionScript)