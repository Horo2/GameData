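; Helper actor in the combat AI folder that moves a target Actor along an arched jump to a given end point.
; On BeginPlay it builds three local XZ control points, raising the midpoint by the jump distance, and turns their Bezier curve into a spline.
; A timeline drives the target along it, sphere-tracing downward late in the jump to stop on ground contact.
; Landing or timeline end fires the complete event after a short delay.
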(event Custom|完成跳跃
  (Utilities|FlowControl|Delay 1.0)
  (Default|CallCompleteEvent))

(event EventBeginPlay
  (bind _returnvalue (Transformation|GetActorTransform))
  (bind _returnvalue_2 (Transformation|GetActorLocation))
  (bind _returnvalue_3 (Transformation|GetActorTransform))
  (bind _returnvalue_4 (Transformation|GetActorLocation))
  (bind _returnvalue_5 (Transformation|GetActorTransform))
  (bind _returnvalue_6 (Math|Conversions|ToFloat(Integer) "2"))
  (bind _returnvalue_7 (Transformation|GetActorTransform))
  (bind _跳跃终点 (Variables|Default|Get跳跃终点))
  (bind _跳跃终点_2 (Variables|Default|Get跳跃终点))
  (bind _actor (Variables|Default|GetActor))
  (bind _returnvalue_8 (Transformation|GetActorLocation _actor))
  (bind _returnvalue_9 (Math|Transform|InverseTransformLocation _returnvalue _跳跃终点))
  (bind _returnvalue_10 (Math|Transform|InverseTransformLocation _returnvalue_3 _returnvalue_2))
  (bind _returnvalue_11 (Math|Transform|InverseTransformLocation _returnvalue_5 _跳跃终点_2))
  (bind _returnvalue_12 (Math|Transform|InverseTransformLocation _returnvalue_7 _returnvalue_4))
  (bind _returnvalue_13 (+ _returnvalue_10 _returnvalue_9))
  (bind _returnvalue_14 (/ _returnvalue_13 _returnvalue_6))
  (Utilities|Array|Clear (Variables|Default|GetSrc))
  (Utilities|Array|Add (Variables|Default|GetSrc) (Math|Vector2D|MakeVector2D (.x _returnvalue_12) (.z _returnvalue_12)))
  (Utilities|Array|Add (Variables|Default|GetSrc) (Math|Vector2D|MakeVector2D (.x _returnvalue_14) (+ (.z _returnvalue_14) (Math|Vector|Distance(Vector) _returnvalue_10 _returnvalue_9))))
  (Utilities|Array|Add (Variables|Default|GetSrc) (Math|Vector2D|MakeVector2D (.x _returnvalue_11) (.z _returnvalue_11)))
  (Spline|ClearSplinePoints (Variables|Default|GetSpline) true)
  (bind _returnvalue_15 (Class|BerzierCurveComponent|BerzierCurve (Variables|Default|GetBerzierCurve) (Variables|Default|GetSrc)))
  (for _array_element _returnvalue_15
    (Spline|AddSplinePoint (Variables|Default|GetSpline) (Math|Vector|MakeVector (.x _array_element) 0.0 (.y _array_element)) "Local" false))
  (Spline|UpdateSpline (Variables|Default|GetSpline))
  (bind _新建轨道_0 (Timeline|时间轴 PlayFromStart)
    (:Update
      (Transformation|SetActorLocation (Variables|Default|GetActor) (Spline|GetLocationatTime (Variables|Default|GetSpline) _新建轨道_0 "World" false) false false)
      (if (> _新建轨道_0 0.8)
        (bind _returnvalue_16 (Collision|SphereTraceByChannel _returnvalue_8 (+ _returnvalue_8 (* (Transformation|GetActorUpVector _actor) (Math|Conversions|ToFloat(Integer) "-100"))) 1e+01 "TraceTypeQuery1" false (Utilities|Array|MakeArray (Variables|Default|GetActor)) "Persistent"))
        (if _returnvalue_16
          (CallFunction|完成跳跃)
          (Timeline|时间轴 Stop))))
    (:Finished
      (CallFunction|完成跳跃))))

(fn ConstructionScript)