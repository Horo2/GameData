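; A single-door Blueprint that slides its Cube upward to open and triggers a CG sequence.
; BeginPlay caches the closed position and an open position raised along Z.
; The AnimationtoDoor event lerps between them using an externally supplied Time alpha.
; On its first call, a DoOnce also spawns BP_CG_Manager, set to trigger on start, passing it the door's CGDataTable.
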(event EventBeginPlay
  (|CallParentFunction)
  (bind _output_get (Variables|Default|Set当前位置 (Variables|/Script/Engine.SceneComponent|GetRelativeLocation (Variables|Default|GetCube))))
  (Variables|Default|Set开门位置 (+ _output_get "0.000000,0.000000,400.000000")))

(event Collision|EventActorBeginOverlap
  (params (OtherActor :type Actor%20Object%20Reference))
  (|CallParentFunction OtherActor) ; 此节点被禁用，将不会被调用。\n从引脚连出引线来编译功能。
)

(event EventTick
  (params (DeltaSeconds :type Float%20%28single-precision%29))
  (|CallParentFunction DeltaSeconds) ; 此节点被禁用，将不会被调用。\n从引脚连出引线来编译功能。
)

(event EventAnimationtoDoor
  (params (Time :type Float%20%28double-precision%29))
  (Transformation|SetRelativeLocation (Variables|Default|GetCube) (Math|Vector|Lerp(Vector) (Variables|Default|Get当前位置) (Variables|Default|Get开门位置) Time) false false)
  (Utilities|FlowControl|DoOnce false
    (:Completed
      (Game|SpawnActorfromClass "/Game/CombatSystem/AVGSystem/BP_CG_Manager.BP_CG_Manager_C" (Math|Transform|MakeTransform "0, 0, 0" "0, 0, 0" "1.000000,1.000000,1.000000") "AlwaysSpawn" "MultiplyWithRoot" 0 0 1 true (Variables|CG|GetCG%20Data%20Table) 0))))

(fn ConstructionScript
  (|CallParentFunction))