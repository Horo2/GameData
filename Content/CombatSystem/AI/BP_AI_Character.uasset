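; BP_AI_Character is an AI-controlled combat NPC that registers itself with BP_AttackManager on BeginPlay.
; A self-restarting delayed loop reads the nav path to the move destination and, on a sufficient rise, jumps and spawns a BP_JumpingCurve, resuming when it completes.
; A repeating timeline turns the NPC toward the player until stopped.
; A cooling component clears the attacking flag, while getters expose NPC data and attack permission.
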(event GeneralAttackCoolingComplete(NPC_CoolingComponents)
  (Variables|Default|SetAttacking false))

(event Custom|Playe%20Rotation%20Animation
  ;[1 1 1] 转身动画
  (Variables|Default|SetIteslf%20Rotation (.yaw (Transformation|GetActorRotation)))
  (bind _新建轨道_0 (Timeline|Turning%20Animation%20Timeline Play)
    (:Update
      (Transformation|SetActorRotation (Math|Rotator|MakeRotator 0.0 0.0 (Math|Float|Lerp (Variables|Default|GetIteslf%20Rotation) (.yaw (Math|Rotator|FindLookatRotation (Transformation|GetActorLocation) (Transformation|GetActorLocation (Game|GetPlayerCharacter 0)))) _新建轨道_0))))
    (:Finished
      (CallFunction|PlayeRotationAnimation))))

(event Custom|Stop%20Rotation%20Animation
  ;[1 1 1] 转身动画
  (bind _新建轨道_0 (Timeline|Turning%20Animation%20Timeline Stop)
    (:Update
      (Transformation|SetActorRotation (Math|Rotator|MakeRotator 0.0 0.0 (Math|Float|Lerp (Variables|Default|GetIteslf%20Rotation) (.yaw (Math|Rotator|FindLookatRotation (Transformation|GetActorLocation) (Transformation|GetActorLocation (Game|GetPlayerCharacter 0)))) _新建轨道_0))))
    (:Finished
      (CallFunction|PlayeRotationAnimation))))

(event Custom|Jumping
  (bind _returnvalue (Transformation|GetActorTransform))
  (Utilities|FlowControl|Delay 0.2)
  (bind _returnvalue_2 (Class|NavigationSystemV1|FindPathtoLocationSynchronously (Transformation|GetActorLocation) (Class|AIController|GetImmediateMoveDestination (AI|GetAIController self)) self 0))
  (Utilities|IsValid _returnvalue_2
    (:Is%20Valid
      (bind _output_get (Variables|Default|SetPath%20Points (Variables|/Script/NavigationSystem.NavigationPath|GetPathPoints _returnvalue_2)))
      (if (== (Utilities|Array|Length _output_get) 2)
        (Utilities|Array|Add (Variables|Default|GetPath%20Points) (* (+ (Utilities|Array|Get(acopy) (Variables|Default|GetPath%20Points)) (Utilities|Array|Get(acopy) (Variables|Default|GetPath%20Points) 1)) (Math|Conversions|ToFloat(Integer) "2")))
        (Utilities|Array|Swap (Variables|Default|GetPath%20Points) 1 2)
        (if (> (- (.z (Utilities|Array|Get(acopy) (Variables|Default|GetPath%20Points) 2)) (.z (Utilities|Array|Get(acopy) (Variables|Default|GetPath%20Points)))) 8e+01) :!label _label
          (Utilities|FlowControl|Delay 0.3)
          (bind _returnvalue_3 (Game|SpawnActorfromClass "/Game/CombatSystem/AI/BP_JumpingCurve.BP_JumpingCurve_C" (Math|Transform|MakeTransform (.location _returnvalue) (.rotation _returnvalue) "1.000000,1.000000,1.000000") "AlwaysSpawn" "MultiplyWithRoot" 0 (Variables|Default|GetPath%20Points) self false "0.000000,0.000000,0.000000" 0))
          (Character|Jump)
          (EventDispatchers|AssignCompleteEvent _returnvalue_3 (delegate Custom|Custom%20Jumping%20Event))
          (else
            (CallFunction|Jumping)))
        (elif (> (Utilities|Array|Length _output_get) 2)
          (goto _label)
          (else
            (CallFunction|Jumping)))))
    (:Is%20Not%20Valid
      (CallFunction|Jumping))))

(event Custom|Custom%20Jumping%20Event
  (CallFunction|Jumping))

(event Custom|Complete%20Event_事件
  (CallFunction|Jumping))

(event EventBeginPlay
  (bind _returnvalue (Actor|GetActorOfClass "/Game/CombatSystem/AI/BP_AttackManager.BP_AttackManager_C"))
  (Utilities|Array|Add (Variables|/Game/CombatSystem/AI/BP_AttackManager.BP_AttackManager_C|GetNPC%20Data _returnvalue) self)
  (CallFunction|Jumping))

(event Collision|EventActorBeginOverlap
  (params (OtherActor :type Actor%20Object%20Reference)))

(event EventTick
  (params (DeltaSeconds :type Float%20%28single-precision%29)))

(fn ConstructionScript)

(fn GetNPCData
  (return (Variables|Default|GetNPC%20Data)))

(fn 获取攻击许可
  (return (Variables|Default|GetAttack%20Permission)))