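; Base combat NPC character that chases the player, waits in attack standby, attacks and pulls back.
; Behaviour events delegate to the data and behaviour management component, which handles status, EQS positioning and attack execution from a configured attack list.
; A looping self-rescue check pathfinds to the player, teleporting the NPC to an EQS escape point on failure unless the player is falling.
; Tick turns the damage-triggered health bar toward the camera and, when enabled, the NPC toward the player.
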(event 伤害通知(C_NPC_DataAndBehaviourManagement_Component)
  (Rendering|SetVisibility (Variables|Default|GetNPC%20Blood%20Strip) true true)
  (Utilities|FlowControl|Delay 4.0)
  (Rendering|SetVisibility (Variables|Default|GetNPC%20Blood%20Strip) false true))

(event Custom|Activation%20NPC
  (Utilities|FlowControl|Delay 0.2)
  (Default|SetNPCStaues (Variables|Default|GetC_NPC_DataAndBehaviourManagement_Component) "NewEnumerator0"))

(event Custom|自救
  (if (not (Variables|Default|Get取消自救))
    (Utilities|FlowControl|Delay 2.0)
    (bind _returnvalue (Class|NavigationSystemV1|FindPathtoLocationSynchronously (Transformation|GetActorLocation) (Transformation|GetActorLocation (Game|Player|GetPlayerPawn 0)) self "/Script/AIModule.NavFilter_AIControllerDefault"))
    (if (Utilities|IsValid _returnvalue)
      (Variables|Default|Set自救半径 1e+02)
      (CallFunction|自救)
      (else
        (bind _returnvalue_2 (AI|EQS|RunEQSQuery "/Game/CombatSystem/AI/EQS/EQS_Escape.EQS_Escape" self "SingleResult" "/Script/AIModule.EnvQueryInstanceBlueprintWrapper"))
        (EventDispatchers|BindEventtoOnQueryFinishedEvent _returnvalue_2 (delegate Custom|自定义事件))))))

(event Custom|完成攻击执行攻击后撤
  ;[0.3333 0 0] NPC 的基础行为脚本
  (Utilities|FlowControl|Delay 0.2)
  (CallFunction|ActivateEnemyService false)
  (Default|攻击后撤 (Variables|Default|GetC_NPC_DataAndBehaviourManagement_Component) "/Game/CombatSystem/AI/EQS/EQS_PullBack.EQS_PullBack" "SingleResult"))

(event Custom|Activate%20Enemy%20Service
  (params (Activate? :type Boolean))
  (Variables|Default|Set看向玩家 Activate?)
  (Variables|Default|SetbUseControllerRotationYaw (not Activate?)))

(event Custom|开始追击玩家
  ;[0.3333 0 0] NPC 的基础行为脚本
  (Utilities|FlowControl|Delay 0.2)
  (CallFunction|ActivateEnemyService false)
  (bind _complete (Default|追击玩家 (Variables|Default|GetC_NPC_DataAndBehaviourManagement_Component) (Game|GetPlayerCharacter 0) "ForOneFrame" :!label _label))
  (if (not _complete)
    (Utilities|FlowControl|Delay 0.2)
    (goto _label)))

(event Custom|设置进入攻击待机
  ;[0.3333 0 0] NPC 的基础行为脚本
  (Utilities|FlowControl|Delay 0.2)
  (Default|SetNPCStaues (Variables|Default|GetC_NPC_DataAndBehaviourManagement_Component) "NewEnumerator3")
  (CallFunction|ActivateEnemyService true))

(event Custom|开始攻击待机
  ;[0.3333 0 0] NPC 的基础行为脚本
  (Utilities|FlowControl|Delay 0.1)
  (if (Default|查询是否在待机范围内 (Variables|Default|GetC_NPC_DataAndBehaviourManagement_Component))
    (bind _npc_attack_licence (Default|查询攻击许可 (Variables|Default|GetC_NPC_DataAndBehaviourManagement_Component)))
    (if _npc_attack_licence
      ;;[1 1 1] 配置攻击能力以及连招
      (CallFunction|QueryConfigurationNPCAttackMode)
      (if (> (Utilities|Array|Length (CallFunction|GetNPCAttackModeData)) (.特殊攻击数量 (CallFunction|QueryAttackDataIsHaveSpecialAttack)))
        (Default|SetNPCStaues (Variables|Default|GetC_NPC_DataAndBehaviourManagement_Component) "NewEnumerator5")
        (else
          (Default|攻击待机 (Variables|Default|GetC_NPC_DataAndBehaviourManagement_Component) "/Game/CombatSystem/AI/EQS/EQS_AttackStandbyLoaction.EQS_AttackStandbyLoaction" "RandomBest25Pct" :!label _label)))
      (else
        (goto _label)))
    (else
      (Default|SetNPCStaues (Variables|Default|GetC_NPC_DataAndBehaviourManagement_Component) "NewEnumerator1"))))

(event Custom|自定义事件
  (params (QueryInstance :type Env%20Query%20Instance%20Blueprint%20Wrapper%20Object%20Reference) (QueryStatus :type EEnvQueryStatus%20Enum :default "Processing"))
  (bind _as角色 (Utilities|Casting|CastToCharacter (Game|Player|GetPlayerPawn 0)))
  (if (not (AI|Components|NavMovement|IsFalling (Variables|/Script/Engine.Character|GetCharacterMovement _as角色)))
    (bind _resultlocations (AI|EQS|GetQueryResultsasLocations QueryInstance))
    (Transformation|SetActorLocation (+ (Utilities|Array|Get(acopy) _resultlocations) "0.000000,0.000000,90.000000") false false)
    (CallFunction|自救)
    (else
      (CallFunction|自救))))

(event Custom|完成攻击待机
  ;[0.3333 0 0] NPC 的基础行为脚本
  (CallFunction|ActivateEnemyService true)
  (if (Default|查询是否在待机范围内 (Variables|Default|GetC_NPC_DataAndBehaviourManagement_Component))
    (Utilities|FlowControl|Delay (.攻击待机间隔 (Utilities|Struct|BreakNPC_CompetenciesData_Structures (Variables|/Game/CombatSystem/NPC/C_NPC_DataAndBehaviourManagement_Component.C_NPC_DataAndBehaviourManagement_Component_C|GetNPC%20Competencies%20Data%20Structures (Variables|Default|GetC_NPC_DataAndBehaviourManagement_Component)))))
    (Default|SetNPCStaues (Variables|Default|GetC_NPC_DataAndBehaviourManagement_Component) "NewEnumerator3")
    (else
      (Default|SetNPCStaues (Variables|Default|GetC_NPC_DataAndBehaviourManagement_Component) "NewEnumerator1"))))

(event Custom|开始攻击玩家
  (params (Idel%20Attack :type Boolean))
  ;[0.3333 0 0] NPC 的基础行为脚本
  (Utilities|FlowControl|Delay 0.2)
  (bind _complete (Default|攻击玩家 (Variables|Default|GetC_NPC_DataAndBehaviourManagement_Component) (Game|GetPlayerCharacter 0) "ForOneFrame" (Utilities|Array|Get(acopy) (CallFunction|GetNPCAttackModeData)) Idel%20Attack :!label _label))
  (if (not _complete)
    (Utilities|FlowControl|Delay 0.1)
    (goto _label)))

(event Custom|执行攻击
  ;[0.3333 0 0] NPC 的基础行为脚本
  (Utilities|FlowControl|Delay 0.2)
  ;;[0 0 0] 开始执行攻击 将配置的攻击数据给到函数会自动进行播放以及处理
  (Default|执行攻击 (Variables|Default|GetC_NPC_DataAndBehaviourManagement_Component) (CallFunction|GetNPCAttackModeData) "None"))

(event Custom|设置进入追击玩家
  (bind _self self)
  ;[0.3333 0 0] NPC 的基础行为脚本
  (if (Variables|Default|GetCG触发中)
    (Animation|StopAnimMontage _self (Animation|GetCurrentMontage _self :!class /Script/Engine.Character))
    (Utilities|FlowControl|Delay 0.2)
    (Default|SetNPCStaues (Variables|Default|GetC_NPC_DataAndBehaviourManagement_Component) "NewEnumerator0")
    (else
      (Default|SetNPCStaues (Variables|Default|GetC_NPC_DataAndBehaviourManagement_Component) "NewEnumerator1"))))

(event EventBeginPlay
  ;[1 0 0] 将NPC同步给血条
  (bind _asnpc_blood_strip (Utilities|Casting|CastToNPC_BloodStrip (UserInterface|GetWidget (Variables|Default|GetNPC%20Blood%20Strip))))
  (Variables|/Game/CombatSystem/NPC/NPC_BloodStrip.NPC_BloodStrip_C|SetNPC%20Character _asnpc_blood_strip self)
  (Rendering|SetVisibility (Variables|Default|GetNPC%20Blood%20Strip) false false)
  (CallFunction|自救))

(event Collision|EventActorBeginOverlap
  (params (OtherActor :type Actor%20Object%20Reference)))

(event EventTick
  (params (DeltaSeconds :type Float%20%28single-precision%29))
  (Transformation|SetWorldRotation (Variables|Default|GetNPC%20Blood%20Strip) (Math|Rotator|FindLookatRotation (Transformation|GetActorLocation) (Transformation|GetActorLocation (Variables|/Script/Engine.PlayerController|GetPlayerCameraManager (Game|GetPlayerController 0)))) false false)
  (if (Variables|Default|Get看向玩家)
    (Transformation|SetActorRotation self (Math|Rotator|MakeRotator 0.0 0.0 (.yaw (Math|Interpolation|RInterpTo (Transformation|GetActorRotation) (Math|Rotator|FindLookatRotation (Transformation|GetActorLocation) (Transformation|GetActorLocation (Game|GetPlayerCharacter 0))) DeltaSeconds (Variables|/Game/CombatSystem/NPC/C_NPC_DataAndBehaviourManagement_Component.C_NPC_DataAndBehaviourManagement_Component_C|GetFollows%20Playeer%20Rotation%20Speed (Variables|Default|GetC_NPC_DataAndBehaviourManagement_Component))))))))

(fn ConstructionScript)

(fn QueryConfigurationNPCAttackMode
  (Utilities|Array|Clear (Variables|Default|GetAttack%20Capability%20Data))
  (return))

(fn GetNPCAttackModeData
  (return (Variables|Default|GetAttack%20Capability%20Data)))

(fn AddNPCAttackModeData
  (params (NewItem :type E_AttackCapabilityConfiguration%20Enum :default "NewEnumerator0"))
  (Utilities|Array|Add (Variables|Default|GetAttack%20Capability%20Data) NewItem)
  (return))

(fn GetNPCAttackAbilityCooldown
  (params (Attack%20Capability :type E_AttackCapabilityConfiguration%20Enum :default "NewEnumerator0"))
  (return (Default|获取某个攻击能力是否正在冷却 (Variables|Default|GetC_NPC_DataAndBehaviourManagement_Component) Attack%20Capability)))

(fn QueryAttackDataIsHaveSpecialAttack
  (LocalVariables|Set记录特殊攻击数量 0)
  (LocalVariables|Set记录查询结果 false)
  (for _array_element (Variables|Default|GetAttack%20Capability%20Data)
    (if (.特殊攻击 (Utilities|Struct|BreakAttackCapabilityDataStructure (.Value (Utilities|Map|Find (Variables|/Game/CombatSystem/NPC/C_NPC_DataAndBehaviourManagement_Component.C_NPC_DataAndBehaviourManagement_Component_C|GetAttack%20Capability%20Configuration (Variables|Default|GetC_NPC_DataAndBehaviourManagement_Component)) _array_element))))
      (LocalVariables|Set记录查询结果 true)
      (Math|Integer|IncrementInt (LocalVariables|Get记录特殊攻击数量))))
  (return (LocalVariables|Get记录查询结果) (LocalVariables|Get记录特殊攻击数量)))