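; CG cutscene manager that plays a storyboard of widgets, triggered on BeginPlay or when the player overlaps its box.
; It disables player input and NPC attack slots, forcing NPC state every Tick during playback.
; Widgets load from a DataTable by incrementing CGID, and sounds are cached per enum from a sound table.
; When no widget remains, or G skips, it stops sounds, restores input and NPCs, then destroys itself.
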(event OnComponentBeginOverlap(Box)
  (params (OverlappedComponent :type Primitive%20Component%20Object%20Reference) (OtherActor :type Actor%20Object%20Reference) (OtherComp :type Primitive%20Component%20Object%20Reference) (OtherBodyIndex :type Integer) (bFromSweep :type Boolean) (SweepResult :type Hit%20Result%20Structure%20%28by%20ref%29))
  (bind _asbp_combat_character_player (Utilities|Casting|CastToBP_CombatCharacter_Player OtherActor))
  (Variables|/Game/CombatSystem/Blueprints/BP_CombatCharacter_Player.BP_CombatCharacter_Player_C|SetBP_CG_Manager _asbp_combat_character_player self)
  (CallFunction|触发CG))

(event OnComponentEndOverlap(Box)
  (params (OverlappedComponent :type Primitive%20Component%20Object%20Reference) (OtherActor :type Actor%20Object%20Reference) (OtherComp :type Primitive%20Component%20Object%20Reference) (OtherBodyIndex :type Integer))
  (bind _asbp_combat_character_player (Utilities|Casting|CastToBP_CombatCharacter_Player OtherActor))
  (Variables|/Game/CombatSystem/Blueprints/BP_CombatCharacter_Player.BP_CombatCharacter_Player_C|SetBP_CG_Manager _asbp_combat_character_player 0))

(event Custom|触发CG
  (bind _returnvalue (Game|GetPlayerController 0))
  (Variables|Default|SetCG已触发 true)
  (bind _outactors (Actor|GetAllActorsOfClass "/Game/CombatSystem/NPC/BP_NPC_ActtackManager.BP_NPC_ActtackManager_C"))
  (for _array_element _outactors
    (Variables|/Game/CombatSystem/NPC/BP_NPC_ActtackManager.BP_NPC_ActtackManager_C|Set已允许攻击的人数 _array_element 0))
  (bind _outactors_2 (Actor|GetAllActorsOfClass "/Game/CombatSystem/NPC/BP_NEW_NPC_Character.BP_NEW_NPC_Character_C"))
  (for _array_element_2 _outactors_2
    (Variables|/Game/CombatSystem/NPC/BP_NEW_NPC_Character.BP_NEW_NPC_Character_C|SetCG触发中 _array_element_2 true)
    (Default|SetNPCStaues (Variables|/Game/CombatSystem/NPC/BP_NEW_NPC_Character.BP_NEW_NPC_Character_C|GetC_NPC_DataAndBehaviourManagement_Component _array_element_2) "NewEnumerator0"))
  (Input|DisableInput _returnvalue _returnvalue)
  (Variables|/Script/Engine.PlayerController|SetbShowMouseCursor _returnvalue true)
  (bind _outrownames (DataTable|GetDataTableRowNames (Variables|数据|GetCG%20Data%20Table)))
  (for _array_element_3 _outrownames
    (bind _returnvalue_2 (Utilities|GetDataTableRow (Variables|数据|GetCG%20Data%20Table) _array_element_3)
      (:then
        (Utilities|Map|Add (Variables|数据|GetCG%20Data) (.CGID (Utilities|Struct|BreakCG_Data_Struct _returnvalue_2)) (.CGWidget (Utilities|Struct|BreakCG_Data_Struct _returnvalue_2))))))
  (CallFunction|StartPlayingCGPicture))

(event Custom|跳过CG
  (Variables|数据|SetCG%20ID 999)
  (CallFunction|EndCGStoryboarding))

(event EventBeginPlay
  (if (Variables|Default|Get开始时触发CG)
    (bind _asbp_combat_character_player (Utilities|Casting|CastToBP_CombatCharacter_Player (Game|Player|GetPlayerPawn 0) :!label _label)
      (:then
        (Variables|/Game/CombatSystem/Blueprints/BP_CombatCharacter_Player.BP_CombatCharacter_Player_C|SetBP_CG_Manager _asbp_combat_character_player self)
        (CallFunction|触发CG))
      (:CastFailed
        (Utilities|FlowControl|Delay 0.2)
        (goto _label)))))

(event EventTick
  (params (DeltaSeconds :type Float%20%28single-precision%29))
  (if (Variables|Default|GetCG已触发)
    (bind _outactors (Actor|GetAllActorsOfClass "/Game/CombatSystem/NPC/BP_NEW_NPC_Character.BP_NEW_NPC_Character_C"))
    (for _array_element _outactors
      (Variables|/Game/CombatSystem/NPC/BP_NEW_NPC_Character.BP_NEW_NPC_Character_C|SetCG触发中 _array_element true)
      (Default|SetNPCStaues (Variables|/Game/CombatSystem/NPC/BP_NEW_NPC_Character.BP_NEW_NPC_Character_C|GetC_NPC_DataAndBehaviourManagement_Component _array_element) "NewEnumerator0"))))

(event EventStartPlayingCGPicture
  (bind _returnvalue (Game|GetPlayerController 0))
  (bind _cg_data (Variables|数据|GetCG%20Data))
  (bind _cg_id (Variables|数据|GetCG%20ID))
  (bind _returnvalue_2 (Utilities|String|ToString(Integer) _cg_id))
  (bind (_value _returnvalue_3) (Utilities|Map|Find _cg_data _returnvalue_2))
  (Utilities|IsValid (Variables|Default|Get当前播放的CG分镜)
    (:Is%20Valid
      (Widget|RemovefromParent (Variables|Default|Get当前播放的CG分镜)))
    (:Is%20Not%20Valid
      _))
  (if _returnvalue_3
    (bind _returnvalue_4 (UserInterface|CreateWidget _value))
    (bind _output_get (Variables|Default|Set当前播放的CG分镜 _returnvalue_4))
    (UserInterface|Viewport|AddtoViewport _output_get 3)
    (Class|AVGSystemInterface|SynchronizeParentClass(Message) (Variables|Default|Get当前播放的CG分镜) self)
    (Class|AVGSystemInterface|StartPlayingCGPicture(Message) (Variables|Default|Get当前播放的CG分镜))
    (else
      (Development|PrintString "已结束CG所有画面" true true "(R=0.000000,G=0.660000,B=1.000000,A=1.000000)" 465465.0)
      (bind _keys (Utilities|Map|Keys (Variables|Default|GetPlaying%20Sound%20Data)))
      (for _array_element _keys
        (Audio|Components|Audio|Stop (.Value (Utilities|Map|Find (Variables|Default|GetPlaying%20Sound%20Data) _array_element))))
      (Variables|/Script/Engine.PlayerController|SetbShowMouseCursor _returnvalue false)
      (Input|EnableInput (Game|Player|GetPlayerPawn 0) _returnvalue)
      (Variables|Default|SetCG已触发 false)
      (Utilities|FlowControl|Delay 0.2)
      (bind _outactors (Actor|GetAllActorsOfClass "/Game/CombatSystem/NPC/BP_NPC_ActtackManager.BP_NPC_ActtackManager_C"))
      (for _array_element_2 _outactors
        (Variables|/Game/CombatSystem/NPC/BP_NPC_ActtackManager.BP_NPC_ActtackManager_C|Set已允许攻击的人数 _array_element_2 3))
      (bind _outactors_2 (Actor|GetAllActorsOfClass "/Game/CombatSystem/NPC/BP_NEW_NPC_Character.BP_NEW_NPC_Character_C"))
      (for _array_element_3 _outactors_2
        (Variables|/Game/CombatSystem/NPC/BP_NEW_NPC_Character.BP_NEW_NPC_Character_C|SetCG触发中 _array_element_3 false)
        (Default|SetNPCStaues (Variables|/Game/CombatSystem/NPC/BP_NEW_NPC_Character.BP_NEW_NPC_Character_C|GetC_NPC_DataAndBehaviourManagement_Component _array_element_3) "NewEnumerator0"))
      (Actor|DestroyActor))))

(event EventEndCGStoryboarding
  (Widget|RemovefromParent (Variables|Default|Get当前播放的CG分镜))
  (Math|Integer|IncrementInt (Variables|数据|GetCG%20ID)
    (:%20%20
      (CallFunction|StartPlayingCGPicture))))

(event EventPlaySound
  (params (SoundEnum :type SoundEnum%20Enum :default "NewEnumerator0") (Stop :type Boolean))
  (bind _playing_sound_data (Variables|Default|GetPlaying%20Sound%20Data))
  (bind _value (Utilities|Map|Find _playing_sound_data SoundEnum))
  (bind (_return_sound_data _return) (CallFunction|获取音频数据 SoundEnum))
  (if _return
    (Utilities|IsValid (.Value (Utilities|Map|Find (Variables|Default|GetPlaying%20Sound%20Data) SoundEnum))
      (:Is%20Valid
        _)
      (:Is%20Not%20Valid
        (bind _returnvalue (Audio|SpawnSound2D (.Sound (Utilities|Struct|BreakSoundStruct _return_sound_data)) 1.0 1.0 0.0 0 false false))
        (Utilities|Map|Add (Variables|Default|GetPlaying%20Sound%20Data) SoundEnum _returnvalue)))
    (if Stop
      (Audio|Components|Audio|Stop _value)
      (else
        (Audio|Components|Audio|Play _value 0.0)))
    (else
      (Development|PrintString "错误！未找到音频文件" true true "(R=1.000000,G=0.000000,B=0.039904,A=1.000000)" 999.0))))

(event Input|KeyboardEvents|G
  (params (Key :type Key%20Structure :default "None"))
  (:Pressed
    (CallFunction|跳过CG)))

(fn ConstructionScript)

(fn 获取音频数据
  (params (Sound%20Enum :type SoundEnum%20Enum :default "NewEnumerator0"))
  (LocalVariables|Set获取 false)
  (bind _outrownames (DataTable|GetDataTableRowNames "/Game/CombatSystem/AVGSystem/Data/CG_Sound_DataTable.CG_Sound_DataTable"))
  (for _array_element _outrownames
    (bind _returnvalue (Utilities|GetDataTableRow "/Game/CombatSystem/AVGSystem/Data/CG_Sound_DataTable.CG_Sound_DataTable" _array_element)
      (:then
        (if (Utilities|Enum|Equal(Enum) (.音频类型 (Utilities|Struct|BreakSoundStruct _returnvalue)) Sound%20Enum)
          (LocalVariables|SetSound%20Data _returnvalue)
          (LocalVariables|Set获取 true)))))
  (if (LocalVariables|Get获取)
    (return (LocalVariables|GetSound%20Data) (LocalVariables|Get获取))
    (else
      (return (Utilities|Struct|MakeSoundStruct "NewEnumerator0" 0) (LocalVariables|Get获取)))))