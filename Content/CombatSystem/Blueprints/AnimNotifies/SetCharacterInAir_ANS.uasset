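; Anim notify state that holds the player combat character at a fixed height for the length of an animation window.
; On begin it has BP_CombatCharacter_Player save its current location.
; Each tick it moves the owner to that saved Z with a swept SetActorLocation, leaving X and Y at their current values.
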(fn ReceivedNotifyTick
  (params (MeshComp :type Skeletal%20Mesh%20Component%20Object%20Reference) (Animation :type Anim%20Sequence%20Base%20Object%20Reference) (FrameDeltaTime :type Float%20%28single-precision%29) (EventReference :type Anim%20Notify%20Event%20Reference%20Structure%20%28by%20ref%29))
  (bind _returnvalue (Components|GetOwner MeshComp))
  (bind _returnvalue_2 (Transformation|GetActorLocation _returnvalue))
  (bind (_x _y) (Math|Vector|BreakVector _returnvalue_2))
  (bind _asbp_combat_character_player (Utilities|Casting|CastToBP_CombatCharacter_Player _returnvalue))
  (Transformation|SetActorLocation _returnvalue (Math|Vector|MakeVector _x _y (.Z (Math|Vector|BreakVector (Default|GetCharacterCurrentLocation _asbp_combat_character_player)))) true false)
  (return false))

(fn ReceivedNotifyBegin
  (params (MeshComp :type Skeletal%20Mesh%20Component%20Object%20Reference) (Animation :type Anim%20Sequence%20Base%20Object%20Reference) (TotalDuration :type Float%20%28single-precision%29) (EventReference :type Anim%20Notify%20Event%20Reference%20Structure%20%28by%20ref%29))
  (bind _asbp_combat_character_player (Utilities|Casting|CastToBP_CombatCharacter_Player (Components|GetOwner MeshComp)))
  (Default|SaveCharacterCurrentLocation _asbp_combat_character_player)
  (return false))