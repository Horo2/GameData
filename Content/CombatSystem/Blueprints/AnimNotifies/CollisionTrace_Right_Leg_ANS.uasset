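; Anim notify state that opens a hit-detection window for right-leg attacks during an animation.
; On begin it fetches the owner's BP_CombatComponent main weapon and enables normal collision tracing on that weapon's right-leg collision component.
; On end it disables the same trace, and both events return false when no valid main weapon exists.
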(fn ReceivedNotifyBegin
  (params (MeshComp :type Skeletal%20Mesh%20Component%20Object%20Reference) (Animation :type Anim%20Sequence%20Base%20Object%20Reference) (TotalDuration :type Float%20%28single-precision%29) (EventReference :type Anim%20Notify%20Event%20Reference%20Structure%20%28by%20ref%29))
  (bind _returnvalue (Components|GetOwner MeshComp))
  (bind _returnvalue_2 (Actor|GetComponentbyClass _returnvalue "/Game/CombatSystem/Blueprints/Components/BP_CombatComponent.BP_CombatComponent_C"))
  (bind _returnvalue_3 (Default|GetMainWeapon _returnvalue_2))
  (Utilities|IsValid _returnvalue_3
    (:Is%20Valid
      (Default|EnableNormalCollisionTrace (Variables|/Game/CombatSystem/Blueprints/Actor/BP_BaseWeapon.BP_BaseWeapon_C|GetBP_Player_Right_Leg_CollisionComponent _returnvalue_3))
      (return true))
    (:Is%20Not%20Valid
      (return false))))

(fn ReceivedNotifyEnd
  (params (MeshComp :type Skeletal%20Mesh%20Component%20Object%20Reference) (Animation :type Anim%20Sequence%20Base%20Object%20Reference) (EventReference :type Anim%20Notify%20Event%20Reference%20Structure%20%28by%20ref%29))
  (bind _returnvalue (Components|GetOwner MeshComp))
  (bind _returnvalue_2 (Actor|GetComponentbyClass _returnvalue "/Game/CombatSystem/Blueprints/Components/BP_CombatComponent.BP_CombatComponent_C"))
  (bind _returnvalue_3 (Default|GetMainWeapon _returnvalue_2))
  (Utilities|IsValid _returnvalue_3
    (:Is%20Valid
      (Default|DisableNormalCollisionTrace (Variables|/Game/CombatSystem/Blueprints/Actor/BP_BaseWeapon.BP_BaseWeapon_C|GetBP_Player_Right_Leg_CollisionComponent _returnvalue_3))
      (return true))
    (:Is%20Not%20Valid
      (return false))))