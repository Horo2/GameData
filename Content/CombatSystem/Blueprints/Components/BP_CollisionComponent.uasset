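; Combat collision component that detects attack hits, attaches impact Niagara effects to hit Characters, plays random hit sounds and broadcasts OnHit.
; While normal collision is enabled, Tick sphere-traces between two sockets on the assigned mesh.
; BoxCollisionTrace, called externally, adds an oriented box component at an owner-relative offset per traceable class and reads overlaps, never destroying the box.
; Both paths share an already-hit list, cleared when collision toggles.
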(event Custom|DisableBoxCollisionTrace
  ;[1 0 0.007892] Disable Collision
  (CallFunction|ClearHitActors)
  (Variables|Default|SetbIsBoxCollisionEnabled? false))

(event Custom|DisableNormalCollisionTrace
  ;[1 0 0.007892] Disable Collision
  (CallFunction|ClearHitActors)
  (Variables|Default|SetbIsCollisionEnabled? false))

(event Custom|CollisionTrace
  (bind _collisionmeshcomponent (Variables|Default|GetCollisionMeshComponent))
  ;[1 0 0.05066] CollisionTrace
  (Variables|Default|SetStart%20Point (Transformation|GetSocketLocation _collisionmeshcomponent (Variables|Initialization|GetStart%20%20Socket%20Name)))
  (Variables|Default|SetEnd%20Point (Transformation|GetSocketLocation _collisionmeshcomponent (Variables|Initialization|GetEnd%20%20Socket%20Name)))
  (bind _outhits (Collision|MultiSphereTraceForObjects (Variables|Default|GetStart%20Point) (Variables|Default|GetEnd%20Point) (Variables|Initialization|GetTraceRadius) (Variables|Initialization|GetCollision%20Object%20Types) false (Variables|初始化|GetActors%20to%20Ignore) (Variables|Initialization|GetDraw%20Debug%20Type)))
  (for _array_element _outhits
    (bind _output_get (Variables|Default|SetLastHit _array_element))
    (if (not (Utilities|Array|ContainsItem (Variables|Default|GetAlreadyHitActors) (.HitActor (Collision|BreakHitResult _output_get))))
      (bind _output_get_2 (Variables|Default|SetHit%20Actor (.HitActor (Collision|BreakHitResult _output_get))))
      (Utilities|Array|Add (Variables|Default|GetAlreadyHitActors) _output_get_2)
      (bind _as角色 (Utilities|Casting|CastToCharacter (.HitActor (Collision|BreakHitResult _output_get))))
      ;;[1 1 1] 攻击命中特效生成
      (Niagara|SpawnSystemAttached (Variables|初始化|Get攻击命中特效) (Variables|/Script/Engine.Character|GetMesh _as角色) "spine_02" (* (Math|Random|RandomUnitVector) 2e+01) (Transformation|GetActorRotation (Variables|Default|GetHit%20Actor)) "KeepRelativeOffset" true)
      ;;[1 1 1] 攻击命中音效
      (Audio|PlaySoundatLocation (.OutItem (Utilities|Array|Random (Variables|初始化|Get攻击命中音效))) (Transformation|GetActorLocation (Components|GetOwner)) "0, 0, 0" (Variables|初始化|Get命中音量) 1.0 0.0 0 0 0 0)
      (Default|CallOnHit :HitActor (Variables|Default|GetHit%20Actor)))))

(event Custom|ClearHitActors
  ;[1 0 0.008526] Clear Hit Actors
  (Utilities|Array|Clear (Variables|Default|GetAlreadyHitActors)))

(event Custom|SetCollisionMesh
  (params (MeshComponent :type Primitive%20Component%20Object%20Reference))
  ;[1 0.01492 0] Set Collision Mesh component
  (Variables|Default|SetCollisionMeshComponent MeshComponent))

(event Custom|BoxCollisionTrace
  (params (Debug%20Mod? :type Boolean) (Box%20Offset%20from%20attacker :type Vector) (Box%20Extent :type Vector))
  (bind _owneractor (Variables|Default|GetOwnerActor))
  (bind _owneractor_2 (Variables|Default|GetOwnerActor))
  (bind _returnvalue (CallFunction|CaclOffset true _owneractor Box%20Offset%20from%20attacker))
  (bind _returnvalue_2 (Transformation|GetActorRotation _owneractor_2))
  ;[1 0 0.05066] CollisionTrace
  (Variables|Default|SetBox%20Extent Box%20Extent)
  (for _array_element (Variables|Default|GetCanTraceActors)
    (bind _out_actors (CallFunction|CrreateBoxCollision _returnvalue _returnvalue_2 (Variables|Default|GetBox%20Extent) _array_element))
    ;;[1 1 1] 测试碰撞范围
    (if Debug%20Mod?
      (Rendering|Debug|DrawDebugBox _returnvalue (Variables|Default|GetBox%20Extent) "(R=1.000000,G=0.033610,B=0.000000,A=1.000000)" _returnvalue_2 1.0 1.0))
    (for _array_element_2 _out_actors
      (if (not (Utilities|Array|ContainsItem (Variables|Default|GetAlreadyHitActors) _array_element_2))
        (bind _output_get (Variables|Default|SetHit%20Actor _array_element_2))
        (Utilities|Array|Add (Variables|Default|GetAlreadyHitActors) _output_get)
        (bind _as角色 (Utilities|Casting|CastToCharacter (Variables|Default|GetHit%20Actor)))
        ;;[1 1 1] 攻击命中特效生成
        (Niagara|SpawnSystemAttached (Variables|初始化|Get攻击命中特效) (Variables|/Script/Engine.Character|GetMesh _as角色) "spine_02" (* (Math|Random|RandomUnitVector) 2e+01) (Transformation|GetActorRotation (Variables|Default|GetHit%20Actor)) "KeepRelativeOffset" true)
        (Audio|PlaySoundatLocation (.OutItem (Utilities|Array|Random (Variables|初始化|Get攻击命中音效))) (Transformation|GetActorLocation (Components|GetOwner)) "0, 0, 0" (Variables|初始化|Get命中音量) 1.0 0.0 0 0 0 0)
        (Default|CallOnHit :HitActor (Variables|Default|GetHit%20Actor))))))

(event Custom|SetOwnerActor
  (params (Owner%20Actor :type Actor%20Object%20Reference))
  ;[1 0 0.008526] Set Owner Actor
  (Variables|Default|SetOwnerActor Owner%20Actor))

(event Custom|EnableNormalCollisionTrace
  ;[1 0 0.01299] Enable Collision
  (CallFunction|ClearHitActors)
  (Variables|Default|SetbIsCollisionEnabled? true))

(event Custom|EnableBoxCollisionTrace
  ;[1 0 0.01299] Enable Collision
  (CallFunction|ClearHitActors)
  (Variables|Default|SetbIsBoxCollisionEnabled? true))

(event EventBeginPlay)

(event EventTick
  (params (DeltaSeconds :type Float%20%28single-precision%29))
  (Utilities|FlowControl|Sequence
    (:then_0
      (if (Variables|Default|GetbIsCollisionEnabled?)
        (CallFunction|CollisionTrace)))))

(fn GetAlereadyHitActors
  (return (Variables|Default|GetAlreadyHitActors)))

(fn IsCollisionEnbaled?
  (return (Variables|Default|GetbIsCollisionEnabled?)))

(fn GetLastHit
  (return (Variables|Default|GetLastHit)))

(fn GetCollisionMeshComponent
  (return (Variables|Default|GetCollisionMeshComponent)))

(fn AddActortoIgnore
  (params (InActor :type Actor%20Object%20Reference%20%28by%20ref%29))
  (Utilities|Array|AddUnique (Variables|初始化|GetActors%20to%20Ignore) InActor))

(fn RemoveActortoIgnore
  (params (ActorToRemove :type Actor%20Object%20Reference%20%28by%20ref%29))
  (Utilities|Array|RemoveItem (Variables|初始化|GetActors%20to%20Ignore) ActorToRemove))

(fn GetActorstoIgnore
  (return (Variables|初始化|GetActors%20to%20Ignore)))

(fn CaclOffset
  (params (AddSelfLocation? :type Boolean) (Actor :type Actor%20Object%20Reference) (Direction :type Vector))
  (return (+ (* (Transformation|GetActorForwardVector Actor) (.x Direction)) (* (Transformation|GetActorRightVector Actor) (.y Direction)) (* (Transformation|GetActorUpVector Actor) (.z Direction)) (Math|Vector|SelectVector (Transformation|GetActorLocation Actor) "0, 0, 0" AddSelfLocation?))))

(fn CrreateBoxCollision
  (params (BoxPosition :type Vector) (BoxRotation :type Rotator) (BoxExtent :type Vector) (ClassFilter :type Actor%20Class%20Reference))
  (bind _returnvalue (Game|AddComponentbyClass (Variables|Default|GetOwnerActor) "/Script/Engine.BoxComponent" false))
  (Transformation|SetWorldLocation _returnvalue BoxPosition false true)
  (Transformation|SetWorldRotation _returnvalue BoxRotation false true)
  (Components|Box|SetBoxExtent _returnvalue BoxExtent true)
  (return (Collision|GetOverlappingActors _returnvalue ClassFilter :!class /Script/Engine.PrimitiveComponent)))