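; Jump-slash sword wave projectile that damages NPCs on behalf of the combat character.
; Each Tick it moves along its Arrow by a fixed per-frame Speed, without sweep or delta-time scaling, and sphere-traces between two marker components, ignoring itself and its owning character.
; On hitting an actor with an NPC data/behaviour component, it sends main-weapon damage and toughness damage scaled by attack-move multipliers, then destroys itself.
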(event EventBeginPlay)

(event Collision|EventActorBeginOverlap
  (params (OtherActor :type Actor%20Object%20Reference)))

(event EventTick
  (params (DeltaSeconds :type Float%20%28single-precision%29))
  (bind _bp_combatchracter (Variables|Default|GetBP_CombatChracter))
  (bind _attack_moes_data (Variables|Default|GetAttack%20Moes%20Data))
  (bind (_actiondamagemultiplier _actiontoughnessdamagemultiplier _attacktypeforhitreflection) (Utilities|Struct|BreakF_AttackMoves _attack_moes_data))
  (bind _combatcomponent (Variables|/Game/CombatSystem/Blueprints/BP_CombatCharacter.BP_CombatCharacter_C|GetCombatComponent _bp_combatchracter))
  (bind _returnvalue (Default|GetMainWeapon _combatcomponent))
  (Transformation|AddActorWorldOffset (* (Math|Vector|GetForwardVector (Variables|Default|GetArrow)) (Variables|Default|GetSpeed)))
  (bind (_outhit _returnvalue_2) (Collision|SphereTraceForObjects (Transformation|GetWorldLocation (Variables|Default|GetState%20Location)) (Transformation|GetWorldLocation (Variables|Default|GetEnd%20Location)) 0.0 (Utilities|Array|MakeArray "ObjectTypeQuery1" "ObjectTypeQuery2" "ObjectTypeQuery3" "ObjectTypeQuery4" "ObjectTypeQuery5" "ObjectTypeQuery6" "ObjectTypeQuery7") false (Utilities|Array|MakeArray self (Variables|Default|GetBP_CombatChracter)) "None"))
  (if _returnvalue_2
    (Utilities|IsValid (Actor|GetComponentbyClass (.HitActor (Collision|BreakHitResult _outhit)) "/Game/CombatSystem/NPC/C_NPC_DataAndBehaviourManagement_Component.C_NPC_DataAndBehaviourManagement_Component_C")
      (:Is%20Valid
        (Class|NPCInteractiveInterface|CreateDamage(Message) (Actor|GetComponentbyClass (.HitActor (Collision|BreakHitResult _outhit)) "/Game/CombatSystem/NPC/C_NPC_DataAndBehaviourManagement_Component.C_NPC_DataAndBehaviourManagement_Component_C") (* (Default|GetBaseDamage _returnvalue) (Math|Float|Clamp(Float) _actiondamagemultiplier 0.01 _actiondamagemultiplier)) (* (Default|GetBaseToughnessDamage _returnvalue) (Math|Float|Clamp(Float) _actiontoughnessdamagemultiplier 0.01 _actiontoughnessdamagemultiplier)) _attacktypeforhitreflection)
        (Actor|DestroyActor)))))

(fn ConstructionScript)