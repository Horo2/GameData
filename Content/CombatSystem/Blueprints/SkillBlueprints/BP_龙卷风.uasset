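; Tornado skill actor that travels forward, repeatedly damaging nearby NPCs and pulling them toward its center.
; A looping timer sphere-traces pawns, deduplicates hits per pulse, applies the caster's weapon damage and toughness damage scaled by attack data, and lerps targets inward.
; Tick moves it along its Arrow unless a line trace finds world objects ahead.
; On destruction it sets a status on NPCs still in radius.
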(event Custom|自定义事件
  (bind _returnvalue (Transformation|GetActorLocation))
  (bind _releases_bp_combatcharacter (Variables|Default|GetReleases%20BP_CombatCharacter))
  (bind _attack_moes_data (Variables|Default|GetAttack%20Moes%20Data))
  (bind (_actiondamagemultiplier _actiontoughnessdamagemultiplier) (Utilities|Struct|BreakF_AttackMoves _attack_moes_data))
  (bind _combatcomponent (Variables|/Game/CombatSystem/Blueprints/BP_CombatCharacter.BP_CombatCharacter_C|GetCombatComponent _releases_bp_combatcharacter))
  (bind _returnvalue_2 (Default|GetMainWeapon _combatcomponent))
  (Utilities|Array|Clear (Variables|Default|GetAlreadyHitActors))
  (bind (_outhits _returnvalue_3) (Collision|MultiSphereTraceForObjects _returnvalue _returnvalue 7.5e+02 (Utilities|Array|MakeArray "ObjectTypeQuery3") false (Utilities|Array|MakeArray self (Variables|Default|GetReleases%20BP_CombatCharacter)) "None"))
  (if _returnvalue_3
    (for _array_element _outhits
      (if (not (Utilities|Array|ContainsItem (Variables|Default|GetAlreadyHitActors) (.HitActor (Collision|BreakHitResult _array_element))))
        (Utilities|Array|Add (Variables|Default|GetAlreadyHitActors) (.HitActor (Collision|BreakHitResult _array_element)))
        (Utilities|IsValid (Actor|GetComponentbyClass (.HitActor (Collision|BreakHitResult _array_element)) "/Game/CombatSystem/NPC/C_NPC_DataAndBehaviourManagement_Component.C_NPC_DataAndBehaviourManagement_Component_C")
          (:Is%20Valid
            (Class|NPCInteractiveInterface|CreateDamage(Message) (Actor|GetComponentbyClass (.HitActor (Collision|BreakHitResult _array_element)) "/Game/CombatSystem/NPC/C_NPC_DataAndBehaviourManagement_Component.C_NPC_DataAndBehaviourManagement_Component_C") (* (Default|GetCurrentDamage _returnvalue_2) (Math|Float|Clamp(Float) _actiondamagemultiplier 0.01 _actiondamagemultiplier)) (* (Default|GetCurrentToughnessDamage _returnvalue_2) (Math|Float|Clamp(Float) _actiontoughnessdamagemultiplier 0.01 _actiontoughnessdamagemultiplier)) "NewEnumerator0")
            (Transformation|SetActorLocation (.HitActor (Collision|BreakHitResult _array_element)) (Math|Vector|Lerp(Vector) (Transformation|GetActorLocation (.HitActor (Collision|BreakHitResult _array_element))) (Transformation|GetActorLocation) 0.1) false false)))))))

(event EventBeginPlay
  (Utilities|Time|SetTimerbyEvent (delegate Custom|自定义事件) 0.1 true))

(event Collision|EventActorBeginOverlap
  (params (OtherActor :type Actor%20Object%20Reference)))

(event EventTick
  (params (DeltaSeconds :type Float%20%28single-precision%29))
  (bind _arrow (Variables|Default|GetArrow))
  (bind _returnvalue (Transformation|GetWorldLocation _arrow))
  (if (not (Variables|Default|GetStop))
    (bind _returnvalue_2 (Collision|LineTraceForObjects _returnvalue (+ _returnvalue (* (Math|Vector|GetForwardVector _arrow) (Math|Conversions|ToVector(Float) 5e+02))) (Utilities|Array|MakeArray "ObjectTypeQuery1" "ObjectTypeQuery2") false (Utilities|Array|MakeArray self 0) "ForDuration"))
    (if (not _returnvalue_2)
      (Transformation|AddActorWorldOffset (* (Math|Vector|GetForwardVector (Variables|Default|GetArrow)) (Variables|Default|GetMove%20Speed))))))

(event EventDestroyed
  (bind _returnvalue (Transformation|GetActorLocation))
  (Variables|Default|SetStop true)
  (bind (_outhits _returnvalue_2) (Collision|MultiSphereTraceForObjects _returnvalue _returnvalue 7.5e+02 (Utilities|Array|MakeArray "ObjectTypeQuery3") false (Utilities|Array|MakeArray self (Variables|Default|GetReleases%20BP_CombatCharacter)) "ForDuration"))
  (if _returnvalue_2
    (for _array_element _outhits
      (Utilities|IsValid (Actor|GetComponentbyClass (.HitActor (Collision|BreakHitResult _array_element)) "/Game/CombatSystem/NPC/C_NPC_DataAndBehaviourManagement_Component.C_NPC_DataAndBehaviourManagement_Component_C")
        (:Is%20Valid
          (Default|SetNPCStaues (Actor|GetComponentbyClass (.HitActor (Collision|BreakHitResult _array_element)) "/Game/CombatSystem/NPC/C_NPC_DataAndBehaviourManagement_Component.C_NPC_DataAndBehaviourManagement_Component_C") "NewEnumerator10"))))))

(fn ConstructionScript)